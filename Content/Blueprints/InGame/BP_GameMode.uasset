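; Game mode that populates the level with NPCs and traps at BeginPlay, using configurable counts.
; Spawn loops place actors at random navmesh-reachable points within a large radius, adjusting for collisions but always spawning.
; NPCs require a successful point lookup, while traps skip that check and use a fixed height.
; CheckPlayerDeath unconditionally flags the supplied PlayerState as dead, despite its name.
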(event `self.ReceiveBeginPlay`
  (`self.SpawnNPC` (`self.SpawnNPCCount`))
  (`self.SpawnTrap` (`self.SpawnTrapCount`)))

(fn `CheckPlayerDeath`
  (params (PlayerState :type "/Game/Blueprints/InGame/Character/BP_PlayerState Object Reference"))
  (set `/Game/Blueprints/InGame/Character/BP_PlayerState.bIsDead` true PlayerState))

(fn `SpawnNPC`
  (params (SpawnNPCCount :type Integer))
  (bind (_randomlocation _returnvalue) (`NavigationSystemV1.K2_GetRandomReachablePointInRadius` (0.0 0.0 90.0) 50000.0 null null))
  (for _ (range 1 (+ SpawnNPCCount 1))
    (if _returnvalue
      (`|SpawnActorFromClass` "/Game/Blueprints/InGame/Character/NPC/BP_NPC.BP_NPC_C" (`KismetMathLibrary.MakeTransform` _randomlocation) "AdjustIfPossibleButAlwaysSpawn" "MultiplyWithRoot" null null))))

(fn `SpawnTrap`
  (params (SpawnTrapCount :type Integer))
  (bind _randomlocation (`NavigationSystemV1.K2_GetRandomReachablePointInRadius` (0.0 0.0 0.0) 50000.0 null null))
  (for _ (range 1 (+ SpawnTrapCount 1))
    (`|SpawnActorFromClass` "/Game/Blueprints/InGame/Character/BP_Trap.BP_Trap_C" (`KismetMathLibrary.MakeTransform` (`KismetMathLibrary.MakeVector` (.x _randomlocation) (.y _randomlocation) 45.0)) "AdjustIfPossibleButAlwaysSpawn" "MultiplyWithRoot" null null)))

(fn `UserConstructionScript`)