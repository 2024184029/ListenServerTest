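; BP_Trap is a spike trap actor that damages players who touch it and knocks them upward.
; When its SprikeTrap component is overlapped and the other actor has authority, it casts to BP_Player, subtracts a fixed amount from CurrentHP and launches the character.
; The death call, S2MServerPlayerDeath, runs only if HP is already depleted on contact, so the hit that empties HP does not itself trigger death.
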(event `self.SprikeTrap.OnComponentBeginOverlap`
  (params (OverlappedComponent :type "PrimitiveComponent Object Reference") (OtherActor :type "Actor Object Reference") (OtherComp :type "PrimitiveComponent Object Reference") (OtherBodyIndex :type Integer) (bFromSweep :type Boolean) (SweepResult :type "HitResult Structure (by ref)"))
  (if (`self.HasAuthority` OtherActor)
    (bind _asbp_player (cast `/Game/Blueprints/InGame/Character/BP_Player` OtherActor))
    (if (> (`/Game/Blueprints/InGame/Character/BP_Player.CurrentHP` _asbp_player) 0.0)
      (set `/Game/Blueprints/InGame/Character/BP_Player.CurrentHP` (- (`/Game/Blueprints/InGame/Character/BP_Player.CurrentHP` _asbp_player) 20.0) _asbp_player)
      (`Character.LaunchCharacter` _asbp_player (0.0 0.0 350.0) false false)
      (else
        (`/Game/Blueprints/InGame/Character/BP_Player.S2M_ServerPlayerDeath` _asbp_player)))))

(fn `UserConstructionScript`)