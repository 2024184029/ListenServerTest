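; BP_Human is a networked human character with a melee attack that kills other humans in one hit.
; CallPowerAttack runs a server-only forward sphere trace with debug drawing and damages each BP_Human hit; CallEndAttack returns the state to IdleMove.
; Damage while idle, moving or attacking triggers S2M_PlayerDeath, which sets Dead, disables movement and capsule collision, and ragdolls the mesh.
; The GameMode and Player casts after death lead to no further logic.
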(event `CallEndAttack`
  ; Attack
  ;; Attack Notify 연결
  (switch `/Game/Blueprints/InGame/Character/EState` (`self.EState`)
    (:`NewEnumerator1`
      (set `self.EState` "NewEnumerator0"))))

(event `CallPowerAttack`
  (bind _returnvalue (`self.K2_GetActorLocation`))
  ; Attack
  ;; Attack Notify 연결
  (`/Engine/EditorBlueprintResources/ActorMacros.Switch Has Authority`
    (:`Authority`
      (bind _outhits (`KismetSystemLibrary.SphereTraceMultiForObjects` :`Start` _returnvalue :`End` (+ _returnvalue (* (`self.GetActorForwardVector`) 200.0)) :`Radius` 20.0 :`ObjectTypes` (`|MakeArray` "ObjectTypeQuery3" :!type "EObjectTypeQuery Enum") :`DrawDebugType` "ForDuration"))
      (for _array_element _outhits
        ;;; Human에게 Damage를 입은 플레이어는 죽음
        (bind _asbp_human (cast `/Game/Blueprints/InGame/Character/BP_Human` (`.HitActor` (`GameplayStatics.BreakHitResult` _array_element))))
        (`GameplayStatics.ApplyDamage` _asbp_human 1.0 null self)))))

(event `self.ReceiveAnyDamage`
  (params (Damage :type "Float (single-precision)") (DamageType :type "DamageType Object Reference") (InstigatedBy :type "Controller Object Reference") (DamageCauser :type "Actor Object Reference"))
  ; Attack
  ;; Human에게 Damage를 입은 플레이어는 죽음
  (switch `/Game/Blueprints/InGame/Character/EState` (`self.EState`)
    (:`NewEnumerator0`
      _)
    (:`NewEnumerator1`
      _))
  (`self.S2M_PlayerDeath`)
  (cast `/Game/Blueprints/InGame/BP_GameMode` (`GameplayStatics.GetGameMode`))
  (cast `/Game/Blueprints/InGame/Character/BP_Player` DamageCauser))

(event `S2M_PlayerDeath`
  (bind _mesh (`self.Mesh`))
  ; Attack
  ;; Human에게 Damage를 입은 플레이어는 죽음
  (set `self.EState` "NewEnumerator2")
  (`CharacterMovementComponent.DisableMovement` (`self.CharacterMovement`))
  (`PrimitiveComponent.SetCollisionEnabled` (`self.CapsuleComponent`) "NoCollision")
  (`PrimitiveComponent.SetCollisionEnabled` _mesh "PhysicsOnly")
  (`PrimitiveComponent.SetSimulatePhysics` _mesh true))

(fn `UserConstructionScript`)