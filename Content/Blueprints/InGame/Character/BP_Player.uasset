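; Networked player character Blueprint that handles attacking, sprinting, death and the in-play UI.
; Attack and sprint input go through C2S to S2M events, with attacks gated to Idle or Move state before playing a montage and sprint switching max walk speed.
; BeginPlay creates and stores the in-play widget.
; The death event disables movement and capsule collision, ragdolls the mesh and shows the game-over widget.
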(event `CallAttackInput`
  ; Attack
  (switch `/Game/Blueprints/InGame/Character/EState` (`self.EState`)
    (:`NewEnumerator0`
      (`self.C2S_Attack`))))

(event `C2S_Attack`
  ; Attack
  (switch `/Game/Blueprints/InGame/Character/EState` (`self.EState`)
    (:`NewEnumerator0`
      (`self.S2M_Attack`))))

(event `S2M_Attack`
  ; Attack
  (set `self.EState` "NewEnumerator1")
  (`self.PlayAnimMontage` "/Game/Assets/Animation/AM_Attack.AM_Attack"))

(event `CallSprintInput`
  (params (IsSprint :type Boolean))
  ; Sprint
  (`self.C2S_Sprint` IsSprint))

(event `C2S_Sprint`
  (params (IsSprint :type Boolean))
  ; Sprint
  (set `self.IsSprint` IsSprint)
  (`self.S2M_Sprint`))

(event `S2M_Sprint`
  (bind _charactermovement (`self.CharacterMovement`))
  ; Sprint
  (if (`self.IsSprint`)
    (set `CharacterMovementComponent.MaxWalkSpeed` 600.0 _charactermovement)
    (else
      (set `CharacterMovementComponent.MaxWalkSpeed` 400.0 _charactermovement))))

(event `self.ReceiveBeginPlay`
  ; UI Ref저장
  (bind _returnvalue (`|CreateWidget` "/Game/Blueprints/InGame/UI/WBP_InPlay.WBP_InPlay_C"))
  (bind _output_get (set `self.UIRef` _returnvalue))
  (`UserWidget.AddToViewport` _output_get 0))

(event `S2M_ServerPlayerDeath`
  (bind _mesh (`self.Mesh`))
  (`CharacterMovementComponent.DisableMovement` (`self.CharacterMovement`))
  (`PrimitiveComponent.SetCollisionEnabled` (`self.CapsuleComponent`) "NoCollision")
  (`PrimitiveComponent.SetCollisionEnabled` _mesh "PhysicsOnly")
  (`PrimitiveComponent.SetSimulatePhysics` _mesh true)
  (bind _returnvalue (`|CreateWidget` "/Game/Blueprints/InGame/UI/WBP_GameOver.WBP_GameOver_C"))
  (`UserWidget.AddToViewport` _returnvalue 0))

(fn `UserConstructionScript`
  (`parent.UserConstructionScript`))